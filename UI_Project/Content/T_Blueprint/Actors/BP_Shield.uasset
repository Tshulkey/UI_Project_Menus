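; BP_Shield is an interactable item actor that adds shield to the player when picked up.
; On interaction it increases the player's Shield by ItemAmount and posts an item notification with the shield icon to the player's HUD.
; The construction script sets a small ItemLimit.
; The IsMaxLimit override flags whether one more shield would reach that limit and returns whether the player is exactly at it.
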(event EventBeginPlay
  (|CallParentFunction) ; This node is disabled and will not be called.\nDrag off pins to build functionality.
)

(event Collision|EventActorBeginOverlap
  (params (OtherActor :type Actor%20Object%20Reference))
  (|CallParentFunction OtherActor) ; This node is disabled and will not be called.\nDrag off pins to build functionality.
)

(event EventTick
  (params (DeltaSeconds :type Float%20%28single-precision%29))
  (|CallParentFunction DeltaSeconds) ; This node is disabled and will not be called.\nDrag off pins to build functionality.
)

(event EventOnActorInteracted
  (params (PlayerReference :type BP%20Third%20Person%20Character%20Object%20Reference))
  (bind _itemamount (Variables|Default|GetItemAmount))
  (Variables|/Game/ThirdPerson/Blueprints/BP_ThirdPersonCharacter.BP_ThirdPersonCharacter_C|SetShield PlayerReference (+ (Variables|/Game/ThirdPerson/Blueprints/BP_ThirdPersonCharacter.BP_ThirdPersonCharacter_C|GetShield PlayerReference) _itemamount))
  (Default|AddItemNotification (Variables|/Game/ThirdPerson/Blueprints/BP_ThirdPersonCharacter.BP_ThirdPersonCharacter_C|GetPlayerHudReference PlayerReference) "Shield" "/Game/UI/PlayerHudAssets/Shield.Shield" _itemamount))

(fn ConstructionScript
  (Variables|Default|SetItemLimit 2))

(fn IsMaxLimit
  (params (PlayerReference :type BP%20Third%20Person%20Character%20Object%20Reference))
  (bind _shield (Variables|/Game/ThirdPerson/Blueprints/BP_ThirdPersonCharacter.BP_ThirdPersonCharacter_C|GetShield PlayerReference))
  (bind _itemlimit (Variables|Default|GetItemLimit))
  ;[0.006278 0.02722 0.15 0.5] Override Function: Checks if the player has the max limit of the item
  (Variables|Default|SetItemLimitReached (>= (+ _shield 1) _itemlimit))
  (return (== _shield _itemlimit)))