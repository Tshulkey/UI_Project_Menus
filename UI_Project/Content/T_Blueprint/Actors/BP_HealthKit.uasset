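; BP_HealthKit is an interactable pickup that restores health to the player character.
; It caches the first player's BP_ThirdPersonCharacter on BeginPlay.
; On interaction, it calls IncreaseHealth on that character's BPCHealthSystem component and destroys itself, but only when health is below maximum.
; An IsMaxLimit function reports whether a given player is at full health, separately from the inline check used on interaction.
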(event EventBeginPlay
  (bind _asbp_third_person_character (Utilities|Casting|CastToBP_ThirdPersonCharacter (Game|GetPlayerCharacter 0)))
  (Variables|Default|SetPlayerReferencee _asbp_third_person_character))

(event EventOnActorInteracted
  (params (PlayerReference :type BP%20Third%20Person%20Character%20Object%20Reference))
  (bind _playerreferencee (Variables|Default|GetPlayerReferencee))
  (bind _bpc_healthsystem (Variables|/Game/ThirdPerson/Blueprints/BP_ThirdPersonCharacter.BP_ThirdPersonCharacter_C|GetBPC_HealthSystem _playerreferencee))
  (if (< (Variables|/Game/ThirdPerson/Blueprints/BPC_HealthSystem.BPC_HealthSystem_C|GetHealth _bpc_healthsystem) (Variables|/Game/ThirdPerson/Blueprints/BPC_HealthSystem.BPC_HealthSystem_C|GetMaxHealth _bpc_healthsystem))
    (Default|IncreaseHealth _bpc_healthsystem (Variables|Default|GetIncreaseHealthAmount))
    (Actor|DestroyActor)))

(fn ConstructionScript
  (|CallParentFunction))

(fn IsMaxLimit
  (params (PlayerReference :type BP%20Third%20Person%20Character%20Object%20Reference))
  (bind _bpc_healthsystem (Variables|/Game/ThirdPerson/Blueprints/BP_ThirdPersonCharacter.BP_ThirdPersonCharacter_C|GetBPC_HealthSystem PlayerReference))
  (return (>= (Variables|/Game/ThirdPerson/Blueprints/BPC_HealthSystem.BPC_HealthSystem_C|GetHealth _bpc_healthsystem) (Variables|/Game/ThirdPerson/Blueprints/BPC_HealthSystem.BPC_HealthSystem_C|GetMaxHealth _bpc_healthsystem))))