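; BP_MasterItems is a base actor for collectible items, with IsMaxLimit meant for child classes to override.
; While under the limit, hovering toggles a custom depth stencil outline, and interacting calls OnActorInteracted, updates the player's HUD item count and destroys the actor.
; A sphere overlap shows the interaction prompt widget unless ItemLimitReached is set, and hides it on exit.
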(event OnComponentBeginOverlap(SphereCollision)
  (params (OverlappedComponent :type Primitive%20Component%20Object%20Reference) (OtherActor :type Actor%20Object%20Reference) (OtherComp :type Primitive%20Component%20Object%20Reference) (OtherBodyIndex :type Integer) (bFromSweep :type Boolean) (SweepResult :type Hit%20Result%20Structure%20%28by%20ref%29))
  ;[0.006278 0.02722 0.15 0.5] Show button Prompt
  ; Interactable Object: When the player overlaps with the interaction sphere we want to set visiblity to true and show the widget. When the overlap ends we want to set visiblity to false and make the widget disappear
  (if (not (Variables|Default|GetItemLimitReached))
    (Rendering|SetVisibility (Variables|Default|GetInteractionPromptWidget) true false)))

(event OnComponentEndOverlap(SphereCollision)
  (params (OverlappedComponent :type Primitive%20Component%20Object%20Reference) (OtherActor :type Actor%20Object%20Reference) (OtherComp :type Primitive%20Component%20Object%20Reference) (OtherBodyIndex :type Integer))
  ;[0.006278 0.02722 0.15 0.5] Show button Prompt
  ; Interactable Object: When the player overlaps with the interaction sphere we want to set visiblity to true and show the widget. When the overlap ends we want to set visiblity to false and make the widget disappear
  (Rendering|SetVisibility (Variables|Default|GetInteractionPromptWidget) false false))

(event Custom|OnActorInteracted
  (params (PlayerReference :type BP%20Third%20Person%20Character%20Object%20Reference))
  ;[0.006278 0.02722 0.15 0.5] Interface Event
  (Utilities|IsValid PlayerReference
    (:Is%20Valid
      (bind _ismax (CallFunction|IsMaxLimit PlayerReference))
      (if (not _ismax)
        (Default|UpdateItemCount (Variables|/Game/ThirdPerson/Blueprints/BP_ThirdPersonCharacter.BP_ThirdPersonCharacter_C|GetPlayerHudReference PlayerReference) PlayerReference)
        (Actor|DestroyActor)))))

(event EventBeginPlay)

(event Collision|EventActorBeginOverlap
  (params (OtherActor :type Actor%20Object%20Reference)))

(event EventTick
  (params (DeltaSeconds :type Float%20%28single-precision%29)))

(event EventOnHovered
  (params (IsHovered :type Boolean) (PlayerReference :type BP%20Third%20Person%20Character%20Object%20Reference))
  ;[0.006278 0.02722 0.15 0.5] Interface Event
  (Utilities|IsValid PlayerReference
    (:Is%20Valid
      (bind _ismax (CallFunction|IsMaxLimit PlayerReference))
      (if (not _ismax)
        (CallFunction|ToggleOutline IsHovered)))))

(event EventOnInteracted
  (params (PlayerReference :type BP%20Third%20Person%20Character%20Object%20Reference))
  ;[0.006278 0.02722 0.15 0.5] Interface Event
  (Utilities|IsValid PlayerReference
    (:Is%20Valid
      (bind _ismax (CallFunction|IsMaxLimit PlayerReference))
      (if (not _ismax)
        (CallFunction|OnActorInteracted PlayerReference)
        (Default|UpdateItemCount (Variables|/Game/ThirdPerson/Blueprints/BP_ThirdPersonCharacter.BP_ThirdPersonCharacter_C|GetPlayerHudReference PlayerReference) PlayerReference)
        (Actor|DestroyActor)))))

(fn ConstructionScript)

(fn ToggleOutline
  (params (IsVisible :type Boolean))
  (bind _staticmesh (Variables|Default|GetStaticMesh))
  (Rendering|SetRenderCustomDepth _staticmesh IsVisible)
  (Rendering|SetCustomDepthStencilValue _staticmesh (Math|Integer|SelectInt 1 0 IsVisible)))

(fn IsMaxLimit
  (params (PlayerReference :type BP%20Third%20Person%20Character%20Object%20Reference))
  ;[0.006278 0.02722 0.15 0.5] Override this function in the child classes
  (return false))