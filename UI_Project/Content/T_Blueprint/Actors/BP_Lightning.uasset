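; BP_Lightning is an interactable pickup that gives the player Lightning items.
; On interaction it adds ItemAmount to the player's Lightning count and posts a HUD item notification with the Spark icon.
; The construction script caps the item at three.
; An IsMaxLimit override reports whether the player is exactly at that cap and sets ItemLimitReached when one more would reach or exceed it.
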(event EventBeginPlay
  (|CallParentFunction) ; This node is disabled and will not be called.\nDrag off pins to build functionality.
)

(event Collision|EventActorBeginOverlap
  (params (OtherActor :type Actor%20Object%20Reference))
  (|CallParentFunction OtherActor) ; This node is disabled and will not be called.\nDrag off pins to build functionality.
)

(event EventTick
  (params (DeltaSeconds :type Float%20%28single-precision%29))
  (|CallParentFunction DeltaSeconds) ; This node is disabled and will not be called.\nDrag off pins to build functionality.
)

(event EventOnActorInteracted
  (params (PlayerReference :type BP%20Third%20Person%20Character%20Object%20Reference))
  (bind _itemamount (Variables|Default|GetItemAmount))
  (Variables|/Game/ThirdPerson/Blueprints/BP_ThirdPersonCharacter.BP_ThirdPersonCharacter_C|SetLightning PlayerReference (+ (Variables|/Game/ThirdPerson/Blueprints/BP_ThirdPersonCharacter.BP_ThirdPersonCharacter_C|GetLightning PlayerReference) _itemamount))
  (Default|AddItemNotification (Variables|/Game/ThirdPerson/Blueprints/BP_ThirdPersonCharacter.BP_ThirdPersonCharacter_C|GetPlayerHudReference PlayerReference) "Lightning" "/Game/UI/Spark.Spark" _itemamount))

(fn ConstructionScript
  (Variables|Default|SetItemLimit 3))

(fn IsMaxLimit
  (params (PlayerReference :type BP%20Third%20Person%20Character%20Object%20Reference))
  (bind _lightning (Variables|/Game/ThirdPerson/Blueprints/BP_ThirdPersonCharacter.BP_ThirdPersonCharacter_C|GetLightning PlayerReference))
  (bind _itemlimit (Variables|Default|GetItemLimit))
  ;[0.006278 0.02722 0.15 0.5] Override Function: Lightning limit is 3 check if the player already has 3
  (Variables|Default|SetItemLimitReached (>= (+ _lightning 1) _itemlimit))
  (return (== _lightning _itemlimit)))